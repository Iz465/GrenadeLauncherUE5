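; BP_MeleeEnemy is a melee enemy that damages the player with a swipe attack.
; While CanHit is set, Tick box-traces between the bone locations behind the mesh's start and end swipe sockets.
; Any blocking hit sends a fixed-damage TakeDamage message to player character 0, without checking the hit actor, then clears CanHit.
; Nothing in these graphs sets CanHit back to true.
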(event EventTick
  (params (DeltaSeconds :type Float%20%28single-precision%29))
  (bind _mesh (Variables|Character|GetMesh))
  (if (Variables|Default|GetCanHit)
    (bind _outhit (Collision|BoxTraceByChannel (Transformation|GetSocketLocation _mesh (Class|SkinnedMeshComponent|GetSocketBoneName _mesh "StartSwipeLocation")) (Transformation|GetSocketLocation _mesh (Class|SkinnedMeshComponent|GetSocketBoneName _mesh "EndSwipeLocation")) "40.000000,20.000000,10.000000" "0, 0, 0" "TraceTypeQuery5" false 0 "None"))
    (if (.bblockinghit _outhit)
      (Class|BPILife|TakeDamage(Message) (Game|GetPlayerCharacter 0) 2e+01 "0, 0, 0")
      (Variables|Default|SetCanHit false))))

(fn ConstructionScript)