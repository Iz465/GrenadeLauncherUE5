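; BP_EnemyManager is an enemy manager Blueprint that, as wired, only caches references and has no working gameplay effect.
; BeginPlay stores the first-person player character and the first BP_GrenadeWeapon1 found in the level, while Tick only checks that the character is valid.
; Disconnected logic would print "Level Complete" once no enemies remain alive, or otherwise kill the player when grenade ammo reaches -1.
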(event EventBeginPlay
  (bind _asbp_first_person_character (Utilities|Casting|CastToBP_FirstPersonCharacter (Game|GetPlayerCharacter 0)))
  (Variables|Default|SetAs%20BP%20First%20Person%20Character _asbp_first_person_character)
  (bind _outactors (Actor|GetAllActorsOfClass "/Game/Items/GrenadeLauncher/BP_GrenadeWeapon1.BP_GrenadeWeapon1_C"))
  (Variables|Default|SetGrenadeWeapon (Utilities|Array|Get(acopy) _outactors)))

(event EventTick
  (params (DeltaSeconds :type Float%20%28single-precision%29))
  (Utilities|IsValid (Variables|Default|GetAs%20BP%20First%20Person%20Character)))

(fn ConstructionScript)