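; Overlap-triggered enemy spawner that starts waves of enemies when the first-person player enters it and moves its bound gate.
; The trigger fires once, placing a BP_EnemySpawn_VFX actor at each valid spawn point and passing it the enemy type and a spawner reference.
; EnemiesAlive spawns the next wave when EnemiesSpawned is empty and waves remain, decrementing WaveAmount.
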(event Custom|SpawnEnemies
  (for _array_element (Variables|Default|GetenemySpawns)
    (Utilities|IsValid _array_element
      (:Is%20Valid
        (bind _returnvalue (Game|SpawnActorfromClass "/Game/Enemies/VFX/BP_EnemySpawn_VFX.BP_EnemySpawn_VFX_C" (Transformation|GetActorTransform _array_element) "Undefined" "MultiplyWithRoot" 0 0))
        (Variables|/Game/Enemies/VFX/BP_EnemySpawn_VFX.BP_EnemySpawn_VFX_C|SetEnemyType _returnvalue (Variables|Default|GetEnemyType))
        (Variables|/Game/Enemies/VFX/BP_EnemySpawn_VFX.BP_EnemySpawn_VFX_C|SetSpawner _returnvalue self)))))

(event Collision|EventActorBeginOverlap
  (params (OtherActor :type Actor%20Object%20Reference))
  (bind _gate_binded (Variables|Default|GetGate%20Binded))
  (if (Variables|Default|GetbCanTrigger)
    (Utilities|Casting|CastToBP_FirstPersonCharacter OtherActor)
    (Variables|Default|SetbCanTrigger false)
    (CallFunction|SpawnEnemies)
    (Utilities|IsValid _gate_binded
      (:Is%20Valid
        (Default|MoveGate _gate_binded (Variables|/Game/Items/Gate/BP_Gate.BP_Gate_C|GetStartLocation _gate_binded) -6e+02)))))

(fn ConstructionScript)

(fn EnemiesAlive
  (if (== (Utilities|Array|Length (Variables|Default|GetEnemiesSpawned)) 0)
    (if (> (Variables|Default|GetWaveAmount) 0)
      (Variables|Default|SetWaveAmount (- (Variables|Default|GetWaveAmount) 1))
      (CallFunction|SpawnEnemies))))