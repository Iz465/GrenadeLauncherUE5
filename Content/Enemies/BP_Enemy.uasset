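; BP_Enemy is an enemy actor that takes damage, bleeds and breaks into body parts when it dies.
; TakeDamage subtracts from the damage field in LifeComponent's life struct, which serves as remaining health, and spawns a Niagara blood splash at the hit location.
; At zero or below, Death spawns a BP_BodyPart at the actor's location for each valid BodyParts mesh, assigns that mesh, then destroys the enemy.
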(event EventDestroyed
  (Development|PrintString "Destroying Enemy"))

(event EventDeath
  (for _array_element (Variables|Default|GetbodyParts)
    (Utilities|IsValid _array_element
      (:Is%20Valid
        (bind _returnvalue (Game|SpawnActorfromClass "/Game/Enemies/BP_BodyPart.BP_BodyPart_C" (Math|Transform|MakeTransform (Transformation|GetActorLocation) "0, 0, 0" "1.000000,1.000000,1.000000") "Undefined" "MultiplyWithRoot" 0 0))
        (Components|StaticMesh|SetStaticMesh (Variables|/Game/Enemies/BP_BodyPart.BP_BodyPart_C|GetBodyMesh _returnvalue) _array_element))))
  (Actor|DestroyActor))

(event EventBeginPlay
  (Development|PrintString "creation of enemy"))

(event EventTakeDamage
  (params (Damage_ :type Float%20%28double-precision%29) (HitLocation :type Vector :default "0, 0, 0"))
  (bind _lifecomponent (Variables|Default|GetlifeComponent))
  (bind _originallifestruct (Variables|/Script/GrenadeLauncherUE5.LifeComponent|GetoriginalLifeStruct _lifecomponent))
  (|SetBy-RefVar (.damage _originallifestruct) (- (.damage _originallifestruct) Damage_))
  (Niagara|SpawnSystematLocation "/Game/Textures/BloodTextures/NS_BloodSplash.NS_BloodSplash" HitLocation)
  (if (<= (.damage _originallifestruct) 0.0)
    (CallFunction|Death)))

(fn ConstructionScript)