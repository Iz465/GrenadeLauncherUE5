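; Gate actor that rises when the first-person character overlaps it, provided its linked Spawner has no enemies in its spawned list or no valid Spawner is set.
; A timeline lerps the actor's location vertically from the GateBottom component's world position to the height of GateTop.
; LowerGate is an empty event, and the lowering timeline is unconnected.
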(event Custom|LowerGate
  (params (Start :type Vector) (End :type Vector)))

(event Custom|RaiseGate
  (params (Start :type Vector) (End :type Vector))
  (bind _newtrack_0 (Timeline|Timeline_0 Play)
    (:Update
      (Transformation|SetActorLocation (Math|Vector|Lerp(Vector) Start (+ Start (Math|Vector|MakeVector 0.0 0.0 (- (.Z (Math|Vector|BreakVector End)) (.Z (Math|Vector|BreakVector Start))))) _newtrack_0) false false))))

(event EventBeginPlay)

(event Collision|EventActorBeginOverlap
  (params (OtherActor :type Actor%20Object%20Reference))
  (bind _spawner (Variables|Default|GetSpawner))
  (Utilities|Casting|CastToBP_FirstPersonCharacter OtherActor)
  (Utilities|IsValid _spawner
    (:Is%20Valid
      (if (== (Utilities|Array|Length (Variables|/Game/Enemies/EnemyManager/BP_EnemySpawner.BP_EnemySpawner_C|GetEnemiesSpawned _spawner)) 0)
        (Variables|Default|SetStartLocation (Transformation|GetWorldLocation (Variables|Default|GetGate%20Bottom)) :!label _label)
        (Variables|Default|SetEndLocation (Transformation|GetWorldLocation (Variables|Default|GetGate%20Top)))
        (CallFunction|RaiseGate (Variables|Default|GetStartLocation) (Variables|Default|GetEndLocation))))
    (:Is%20Not%20Valid
      (goto _label))))

(fn ConstructionScript)