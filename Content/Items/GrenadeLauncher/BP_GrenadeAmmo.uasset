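; Grenade launcher ammo actor that shatters Chaos Geometry Collection objects it hits.
; On its first hit it turns on mesh physics, then applies massive external strain and a radial impulse at the impact point of any Geometry Collection found.
; The ammo mesh then hides and a timer destroys the fractured actor seconds later, while the ammo actor itself remains.
; Hits on anything else destroy the ammo immediately.
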(event Custom|RemoveDebris
  (Development|PrintString "destroying")
  (for _array_element (Variables|Default|GetDestroyedDebris)
    (Actor|DestroyActor _array_element)))

(event EventBeginPlay)

(event Collision|EventActorBeginOverlap
  (params (OtherActor :type Actor%20Object%20Reference)))

(event EventTick
  (params (DeltaSeconds :type Float%20%28single-precision%29)))

(event Collision|EventHit
  (params (MyComp :type Primitive%20Component%20Object%20Reference) (Other :type Actor%20Object%20Reference) (OtherComp :type Primitive%20Component%20Object%20Reference) (bSelfMoved :type Boolean) (HitLocation :type Vector :default "0, 0, 0") (HitNormal :type Vector :default "0, 0, 0") (NormalImpulse :type Vector :default "0, 0, 0") (Hit :type Hit%20Result%20Structure%20%28by%20ref%29))
  (bind _returnvalue (Actor|GetComponentbyClass Other "/Script/GeometryCollectionEngine.GeometryCollectionComponent"))
  (Utilities|FlowControl|DoOnce false
    (:Completed
      (Physics|SetSimulatePhysics (Variables|Default|GetammoMesh) true)
      (Utilities|IsValid _returnvalue
        (:Is%20Valid
          (bind _output_get (Variables|/Script/GeometryCollectionEngine.GeometryCollectionComponent|SetbEnableDamageFromCollision _returnvalue true))
          (if _output_get
            (Development|PrintString (Utilities|GetDisplayName _returnvalue))
            (Class|GeometryCollectionComponent|ApplyExternalStrain _returnvalue 0 HitLocation 3e+12 10 2.0 1e+67)
            (Physics|AddRadialImpulse _returnvalue HitLocation 3e+06 2e+03 "RIF_Constant" true)
            (Development|PrintString "...................")
            (Rendering|SetVisibility (Variables|Default|GetammoMesh) false false)
            (Utilities|Array|Add (Variables|Default|GetDestroyedDebris) (Components|GetOwner _returnvalue))
            (Utilities|Time|SetTimerbyEvent (delegate Custom|RemoveDebris) 3.0)))
        (:Is%20Not%20Valid
          (Actor|DestroyActor))))))

(fn ConstructionScript)