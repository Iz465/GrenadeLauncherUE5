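; BP_GrenadeWeapon1 is a grenade launcher weapon Blueprint that tracks the player's aim while charging.
; BeginPlay caches the first-person character, and Tick sets LaunchVelocity to the camera's forward vector, unscaled, while Charging is true.
; A disconnected branch, which never runs, ramps clamped height and distance, builds an arced velocity and debug-draws the predicted projectile path.
; StartShake is an empty event.
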(event EventBeginPlay
  (bind _asbp_first_person_character (Utilities|Casting|CastToBP_FirstPersonCharacter (Game|GetPlayerCharacter 0)))
  (Variables|Default|SetAs%20BP%20First%20Person%20Character _asbp_first_person_character))

(event Collision|EventActorBeginOverlap
  (params (OtherActor :type Actor%20Object%20Reference)))

(event EventTick
  (params (DeltaSeconds :type Float%20%28single-precision%29))
  (if (Variables|Default|Getcharging)
    (Variables|Default|SetlaunchVelocity (Math|Vector|GetForwardVector (Variables|/Script/GrenadeLauncherUE5.GrenadeLauncherUE5Character|GetFirstPersonCameraComponent (Variables|Default|GetAs%20BP%20First%20Person%20Character))))))

(event EventStartShake)

(fn ConstructionScript)