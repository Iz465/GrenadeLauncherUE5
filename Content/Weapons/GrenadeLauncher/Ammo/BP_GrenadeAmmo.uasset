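; BP_GrenadeAmmo is the grenade launcher's ammo actor, applying damage and a Niagara effect on impact.
; Its Hit event sends the owning weapon's damage to the hit actor via TakeDamageMessage, spawns the effect, enables mesh physics and immediately destroys itself.
; The whole reaction depends on a BP_FPS_GameInstance cast, whose saved damage is only debug-printed.
; Damage hits only that actor, with no radius check.
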(event Collision|EventHit
  (params (MyComp :type Primitive%20Component%20Object%20Reference) (Other :type Actor%20Object%20Reference) (OtherComp :type Primitive%20Component%20Object%20Reference) (bSelfMoved :type Boolean) (HitLocation :type Vector :default "0, 0, 0") (HitNormal :type Vector :default "0, 0, 0") (NormalImpulse :type Vector :default "0, 0, 0") (Hit :type Hit%20Result%20Structure%20%28by%20ref%29))
  (bind _asbp_fps_game_instance (Utilities|Casting|CastToBP_FPS_GameInstance (Game|GetGameInstance)))
  (Class|BPILife|TakeDamage(Message) Other (.damage (Utilities|Struct|BreakWeaponInfo (Variables|/Script/GrenadeLauncherUE5.Weapons|GetweaponInfo (Variables|Default|Getweapon)))) HitLocation)
  (Development|PrintString (Utilities|String|ToString(Float) (.damage (Utilities|Struct|BreakSavedWeaponInfo (Variables|/Script/GrenadeLauncherUE5.FPS_GameInstance|GetsavedWeaponInfo _asbp_fps_game_instance)))))
  (Niagara|SpawnSystematLocation "/Game/Basic_VFX/Niagara/NS_Basic_2.NS_Basic_2" HitLocation)
  (Physics|SetSimulatePhysics (Variables|Default|GetammoMesh) true)
  (Actor|DestroyActor))

(fn ConstructionScript)