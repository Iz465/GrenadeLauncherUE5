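; Grenade launcher weapon Blueprint that handles its own reload and stubs out perk hooks.
; When ammo is below the GameInstance's saved amount, reload refills it and plays the first-person montage at the saved reload speed.
; Montage notifies spawn a grenade mesh actor attached to the left hand, then destroy it.
; Value-increase and element functions only print debug strings, while value-decrease is empty.
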(event EventReloadAnimation
  (bind _player (Variables|Default|Getplayer))
  (bind _weaponinfo (Variables|Default|GetweaponInfo))
  (bind _gameinstance (Variables|Default|GetgameInstance))
  (bind _savedweaponinfo (Variables|/Script/GrenadeLauncherUE5.FPS_GameInstance|GetsavedWeaponInfo _gameinstance))
  (bind (_name _damage _ammo _reloadspeedrate) (Utilities|Struct|BreakSavedWeaponInfo _savedweaponinfo))
  (if (< (.ammo _weaponinfo) _ammo)
    (|SetBy-RefVar (.ammo _weaponinfo) _ammo)
    (Variables|Default|SethasReloaded false)
    (Utilities|IsValid _player
      (:Is%20Valid
        (bind _notifyname (Animation|Montage|PlayMontage (Variables|/Script/GrenadeLauncherUE5.GrenadeLauncherUE5Character|GetMesh1P _player) "/Game/Adventurer/Animation/AM_GrenadeLauncher.AM_GrenadeLauncher" _reloadspeedrate 0.0 "Reload")
          (:OnNotifyBegin
            ;[0.15 0.15 0.15 0.5] Not Generic - Used for spawning the ammo in the reload animation
            (Utilities|FlowControl|Sequence
              (:then_0
                (if (== (Utilities|Name|MakeLiteralName _notifyname) "SpawnAmmo")
                  (bind _returnvalue (Game|SpawnActorfromClass "/Script/Engine.StaticMeshActor" (Math|Transform|MakeTransform "3.890000,-2.970000,4.660000" "36.530000,-74.560000,-91.180000" "0.400000,0.400000,0.400000") "Undefined" "MultiplyWithRoot" 0 0))
                  (Variables|Default|SetAmmo%20Mesh _returnvalue)
                  (Collision|SetCollisionEnabled (Variables|/Script/Engine.StaticMeshActor|GetStaticMeshComponent _returnvalue) "NoCollision")
                  (Transformation|SetMobility (Variables|/Script/Engine.StaticMeshActor|GetStaticMeshComponent _returnvalue) "Movable")
                  (Components|StaticMesh|SetStaticMesh (Variables|/Script/Engine.StaticMeshActor|GetStaticMeshComponent _returnvalue) "/Game/Weapons/GrenadeLauncher/Ammo/GrenadeAmmo.GrenadeAmmo")
                  (Transformation|AttachComponentToComponent _returnvalue (Variables|/Script/GrenadeLauncherUE5.GrenadeLauncherUE5Character|GetMesh1P (Variables|Default|Getplayer)) "LeftHand" "KeepRelative" "KeepRelative" "KeepRelative" true)))
              (:then_1
                (if (== (Utilities|Name|MakeLiteralName _notifyname) "DestroyAmmo")
                  (Actor|DestroyActor (Variables|Default|GetAmmo%20Mesh)))))))))))

(fn ConstructionScript)

(fn IncreaseWeaponValues
  (params (Min%20Value :type Float%20%28double-precision%29) (Max%20Value :type Float%20%28double-precision%29) (Value%20Cap :type Float%20%28double-precision%29))
  (Development|PrintString "INCREASING VALUE ON WEAPON" true true "(R=1.000000,G=0.000000,B=0.003372,A=1.000000)"))

(fn DecreaseWeaponValues
  (params (Min%20Value :type Float%20%28double-precision%29) (Max%20Value :type Float%20%28double-precision%29) (Value%20Cap :type Float%20%28double-precision%29)))

(fn ApplyElement
  (params (Perk%20Enum :type EPerkName%20Enum :default "damage"))
  (switch Utilities|FlowControl|Switch|SwitchonEPerkName Perk%20Enum
    (:freeze
      (Development|PrintString "FREEZING" true true "(R=0.018216,G=0.007232,B=1.000000,A=1.000000)"))
    (:poison
      (Development|PrintString "POISONING" true true "(R=0.031783,G=1.000000,B=0.000000,A=1.000000)"))
    (:burn
      (Development|PrintString "BURNING" true true "(R=1.000000,G=0.256820,B=0.000000,A=1.000000)"))))