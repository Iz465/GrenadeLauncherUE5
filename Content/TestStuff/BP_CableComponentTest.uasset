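; Test actor, by its name for a cable component, that moves a Hook component along an arced cast path to EndObject.
; Five seconds after BeginPlay, a Timeline lerps the Hook from its starting location to EndObject's current location.
; A half sine wave adds vertical lift, scaled by Castheight, a fraction of a distance to EndObject.
; Castheight is computed before Start is set to the Hook's location, so it uses Start's prior value.
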(event EventBeginPlay
  (Variables|Default|Setcastheight (* (Math|Vector|Distance(Vector) (Variables|Default|GetStart) (Transformation|GetActorLocation (Variables|Default|GetEndObject))) 0.3))
  (Variables|Default|SetStart (Transformation|GetWorldLocation (Variables|Default|GetHook)))
  (Utilities|FlowControl|Delay 5.0)
  (bind _newtrack_0 (Timeline|Timeline Play)
    (:Update
      (Transformation|SetWorldLocation (Variables|Default|GetHook) (Math|Vector|MakeVector (.x (Math|Vector|Lerp(Vector) (Variables|Default|GetStart) (Transformation|GetActorLocation (Variables|Default|GetEndObject)) _newtrack_0)) (.y (Math|Vector|Lerp(Vector) (Variables|Default|GetStart) (Transformation|GetActorLocation (Variables|Default|GetEndObject)) _newtrack_0)) (+ (* (Math|Trig|Sin(Radians) (Math|Float|MultiplybyPi _newtrack_0)) (Variables|Default|Getcastheight)) (.z (Math|Vector|Lerp(Vector) (Variables|Default|GetStart) (Transformation|GetActorLocation (Variables|Default|GetEndObject)) _newtrack_0)))) false false))))

(event EventTick
  (params (DeltaSeconds :type Float%20%28single-precision%29)))

(fn ConstructionScript)