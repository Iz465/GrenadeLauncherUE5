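; Test Blueprint that builds collidable spline meshes between its Start and End actors.
; Every Tick it adds a new spline mesh per spline point without removing old ones, so components accumulate.
; Each spans the two actors' world locations, taking its start tangent from point 0 and end tangent from the next point.
; A point-to-point segment builder in the construction script is disconnected and never runs.
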(event EventBeginPlay)

(event EventTick
  (params (DeltaSeconds :type Float%20%28single-precision%29))
  (bind _spline (Variables|Default|GetSpline))
  (for _index (range 0 (Spline|GetNumberOfSplinePoints (Variables|Default|GetSpline)))
    (bind _returnvalue (AddComponent|AddSplineMeshComponent false))
    (Development|PrintString "CREATED")
    (SplineMesh|SetForwardAxis _returnvalue "Z" true)
    (SplineMesh|SetStartandEnd _returnvalue (Transformation|GetActorLocation (Variables|Default|GetStart)) (Spline|GetTangentatSplinePoint _spline 0 "Local") (Transformation|GetActorLocation (Variables|Default|GetEnd)) (Spline|GetTangentatSplinePoint _spline (+ _index 1) "Local") true :!class /Script/Engine.SplineMeshComponent)
    (Collision|SetCollisionEnabled _returnvalue "QueryAndPhysics")))

(fn ConstructionScript)